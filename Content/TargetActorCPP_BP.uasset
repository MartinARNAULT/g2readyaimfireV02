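; Shootable target actor that awards score when a bullet hits it and tracks how many targets remain.
; It caches the Player_Pawn on BeginPlay, and a hit on its Cylinder by a Bullet_Actor destroys the bullet, adds to the pawn's Score and decrements its TotalTarget.
; The target destroys itself while targets remain, and opens Game_Level when the count runs out.
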(event `self.ReceiveBeginPlay`
  (bind _asplayer_pawn (cast `/Game/Player_Pawn` (`GameplayStatics.GetPlayerPawn` 0)))
  (set `self.Player_Pawn` _asplayer_pawn))

(event `self.Cylinder.OnComponentHit`
  (params (HitComponent :type "PrimitiveComponent Object Reference") (OtherActor :type "Actor Object Reference") (OtherComp :type "PrimitiveComponent Object Reference") (NormalImpulse :type "Vector Structure") (Hit :type "HitResult Structure (by ref)"))
  (bind _player_pawn (`self.Player_Pawn`))
  (if (`KismetMathLibrary.ClassIsChildOf` (`GameplayStatics.GetObjectClass` OtherActor) "/Game/Bullet_Actor.Bullet_Actor_C")
    (`self.K2_DestroyActor` OtherActor)
    (set `/Game/Player_Pawn.Score` (+ (`/Game/Player_Pawn.Score` _player_pawn) 100) _player_pawn)
    (bind _result (`/Engine/EditorBlueprintResources/StandardMacros.DecrementInt` (`/Game/Player_Pawn.Total Target` (`self.Player_Pawn`)))
      (:`  `
        (if (<= _result 0)
          (`GameplayStatics.OpenLevel` "Game_Level")
          (else
            (`self.K2_DestroyActor`)))))))

(fn `UserConstructionScript`)